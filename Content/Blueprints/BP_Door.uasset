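; Door actor that plays a sound and slows the SpiritFrequencyCharacter while it overlaps the door.
; Begin overlap lowers the character's max walk speed, and end overlap sets it to a fixed faster value rather than the saved original.
; Both events add an audio component, then share one play-sound-at-location call at the door's position.
; The graph contains no logic that opens or moves the door.
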(event `self.ReceiveActorBeginOverlap`
  (params (OtherActor :type "Actor Object Reference"))
  (bind _asspirit_frequency_character (cast `SpiritFrequencyCharacter` OtherActor))
  (`|ExecutionSequence`
    (:`then_0`
      (`AddComponent|NODE_AddAudioComponent-0`)
      (`GameplayStatics.PlaySoundAtLocation` null (`self.K2_GetActorLocation`) (struct) 1.0 1.0 0.0 null null null null :!label _label))
    (:`then_1`
      (set `CharacterMovementComponent.MaxWalkSpeed` 100.0 (`Character.CharacterMovement` _asspirit_frequency_character)))))

(event `self.ReceiveActorEndOverlap`
  (params (OtherActor :type "Actor Object Reference"))
  (bind _asspirit_frequency_character (cast `SpiritFrequencyCharacter` OtherActor))
  (`|ExecutionSequence`
    (:`then_0`
      (`AddComponent|NODE_AddAudioComponent-1`)
      (goto _label))
    (:`then_1`
      (set `CharacterMovementComponent.MaxWalkSpeed` 300.0 (`Character.CharacterMovement` _asspirit_frequency_character)))))

(fn `UserConstructionScript`)